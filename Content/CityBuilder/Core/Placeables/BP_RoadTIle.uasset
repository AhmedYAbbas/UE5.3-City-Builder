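; BP_RoadTIle is the placeable road tile for the city builder, adjusting its four sides to the surrounding grid.
; When OnNewRoadTileAdded fires, it calls UpdateSideOfRoadTile once per side, pairing each neighbour of its grid cell with the North, East, South or West pathway.
; The per-side update logic is not defined in this graph, and the construction script is empty.
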(event `self.OnNewRoadTileAdded`
  (`self.UpdateSideOfRoadTile` (`|GetArrayItem` (`CBGridCell.Neighbours` (`self.GridCellRef`))) (`self.PathwayNorth`))
  (`self.UpdateSideOfRoadTile` (`|GetArrayItem` (`CBGridCell.Neighbours` (`self.GridCellRef`)) 1) (`self.PathwayEast`))
  (`self.UpdateSideOfRoadTile` (`|GetArrayItem` (`CBGridCell.Neighbours` (`self.GridCellRef`)) 2) (`self.PathwaySouth`))
  (`self.UpdateSideOfRoadTile` (`|GetArrayItem` (`CBGridCell.Neighbours` (`self.GridCellRef`)) 3) (`self.PathwayWest`)))

(fn `UserConstructionScript`)