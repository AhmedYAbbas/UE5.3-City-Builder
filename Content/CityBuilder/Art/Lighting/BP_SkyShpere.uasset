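; Sky sphere Blueprint for the city builder's lighting, deferring construction to its parent class.
; On BeginPlay it caches its directional light actor as the sun and finds the BP_TimeManager in the level.
; Logic to pitch the sun from the manager's time of day and update sun direction exists but is disconnected; Tick does nothing.
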(event `self.ReceiveBeginPlay`
  (set `self.Sun` (`self.Directional light actor`))
  (bind _returnvalue (`GameplayStatics.GetActorOfClass` "/Game/CityBuilder/Core/Time/BP_TimeManager.BP_TimeManager_C"))
  (set `self.TimeManager` _returnvalue))

(event `self.ReceiveTick`
  (params (DeltaSeconds :type "Float (single-precision)")))

(fn `UserConstructionScript`
  (`parent.UserConstructionScript`))